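; BP_ClientSocket is the client socket Blueprint for the login map, pushing user, room and chat text into the login UI.
; Three upload events each wrap a string in a new ChatLine widget, append it to the matching list and scroll to the end.
; OffLoginUI switches the screen from login to lobby by toggling widget visibility and shows the PlayerID read from BP_ChatGameModeBase.
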(event `self.UploadUserList`
  (params (chat :type String))
  (bind _userlist (`/Game/Maps/Login/BP_Login.UserList` (`/Game/Maps/Login/BP_UIManager.bp_login` (`self.LoginUI`))))
  (bind _returnvalue (`|CreateWidget` "/Game/ChatLine.ChatLine_C"))
  (`/Game/ChatLine.Init Text` _returnvalue chat)
  (`PanelWidget.AddChild` _userlist _returnvalue)
  (`ScrollBox.ScrollToEnd` _userlist))

(event `self.UploadRoomList`
  (params (chat :type String))
  (bind _roomlist (`/Game/Maps/Login/BP_Login.RoomList` (`/Game/Maps/Login/BP_UIManager.bp_login` (`self.LoginUI`))))
  (bind _returnvalue (`|CreateWidget` "/Game/ChatLine.ChatLine_C"))
  (`/Game/ChatLine.Init Text` _returnvalue chat)
  (`PanelWidget.AddChild` _roomlist _returnvalue)
  (`ScrollBox.ScrollToEnd` _roomlist))

(event `self.UploadChat`
  (params (chat :type String))
  (bind _lobbychatbox (`/Game/Maps/Login/BP_Login.LobbyChatBox` (`/Game/Maps/Login/BP_UIManager.bp_login` (`self.LoginUI`))))
  (bind _returnvalue (`|CreateWidget` "/Game/ChatLine.ChatLine_C"))
  (`/Game/ChatLine.Init Text` _returnvalue chat)
  (`PanelWidget.AddChild` _lobbychatbox _returnvalue)
  (`ScrollBox.ScrollToEnd` _lobbychatbox))

(event `self.OffLoginUI`
  (bind _bp_login (`/Game/Maps/Login/BP_UIManager.bp_login` (`self.LoginUI`)))
  (bind _defaulidui (`/Game/Maps/Login/BP_Login.defaulIDUI` _bp_login))
  (`Widget.SetVisibility` (`/Game/Maps/Login/BP_Login.InputIP` (`/Game/Maps/Login/BP_UIManager.bp_login` (`self.LoginUI`))) "Hidden")
  (`Widget.SetVisibility` (`/Game/Maps/Login/BP_Login.Button_Enter` (`/Game/Maps/Login/BP_UIManager.bp_login` (`self.LoginUI`))) "Hidden")
  (`Widget.SetVisibility` (`/Game/Maps/Login/BP_Login.InputID_BackGround` (`/Game/Maps/Login/BP_UIManager.bp_login` (`self.LoginUI`))) "Hidden")
  (`Widget.SetVisibility` (`/Game/Maps/Login/BP_Login.InputID` (`/Game/Maps/Login/BP_UIManager.bp_login` (`self.LoginUI`))) "Hidden")
  (`Widget.SetVisibility` (`/Game/Maps/Login/BP_Login.Button_Server` (`/Game/Maps/Login/BP_UIManager.bp_login` (`self.LoginUI`))) "Hidden")
  (`Widget.SetVisibility` (`/Game/Maps/Login/BP_Login.InputIP_BackGround` (`/Game/Maps/Login/BP_UIManager.bp_login` (`self.LoginUI`))) "Hidden")
  (`Widget.SetVisibility` (`/Game/Maps/Login/BP_Login.IDUI` _bp_login) "Visible")
  (`Widget.SetVisibility` (`/Game/Maps/Login/BP_Login.PosUI` _bp_login) "Visible")
  (`Widget.SetVisibility` (`/Game/Maps/Login/BP_Login.DefaultPosUI` _bp_login) "Visible")
  (bind _asbp_chat_game_mode_base (cast `/Game/BluePrint/BP_ChatGameModeBase` (`GameplayStatics.GetGameMode`)))
  (`TextBlock.SetText` _defaulidui (`KismetTextLibrary.Conv_StringToText` (`/Game/BluePrint/BP_ChatGameModeBase.PlayerID` _asbp_chat_game_mode_base)))
  (`Widget.SetVisibility` _defaulidui "Visible")
  (`Widget.SetVisibility` (`/Game/Maps/Login/BP_Login.PosName` (`/Game/Maps/Login/BP_UIManager.bp_login` (`self.LoginUI`))) "Visible")
  (`Widget.SetVisibility` (`/Game/Maps/Login/BP_Login.LobbyChatBackGround` (`/Game/Maps/Login/BP_UIManager.bp_login` (`self.LoginUI`))) "Visible")
  (`Widget.SetVisibility` (`/Game/Maps/Login/BP_Login.LobbyChatBox` (`/Game/Maps/Login/BP_UIManager.bp_login` (`self.LoginUI`))) "Visible")
  (`Widget.SetVisibility` (`/Game/Maps/Login/BP_Login.LobbyChatSendButton` (`/Game/Maps/Login/BP_UIManager.bp_login` (`self.LoginUI`))) "Visible")
  (`Widget.SetVisibility` (`/Game/Maps/Login/BP_Login.LobbyInputChat` (`/Game/Maps/Login/BP_UIManager.bp_login` (`self.LoginUI`))) "Visible")
  (`Widget.SetVisibility` (`/Game/Maps/Login/BP_Login.RoomList` (`/Game/Maps/Login/BP_UIManager.bp_login` (`self.LoginUI`))) "Visible")
  (`Widget.SetVisibility` (`/Game/Maps/Login/BP_Login.EnterRoomButton` (`/Game/Maps/Login/BP_UIManager.bp_login` (`self.LoginUI`))) "Visible")
  (`Widget.SetVisibility` (`/Game/Maps/Login/BP_Login.ListRoomButton` (`/Game/Maps/Login/BP_UIManager.bp_login` (`self.LoginUI`))) "Visible")
  (`Widget.SetVisibility` (`/Game/Maps/Login/BP_Login.MakeRoomButton` (`/Game/Maps/Login/BP_UIManager.bp_login` (`self.LoginUI`))) "Visible")
  (`Widget.SetVisibility` (`/Game/Maps/Login/BP_Login.List` (`/Game/Maps/Login/BP_UIManager.bp_login` (`self.LoginUI`))) "Visible")
  (`Widget.SetVisibility` (`/Game/Maps/Login/BP_Login.RoolListBackGround` (`/Game/Maps/Login/BP_UIManager.bp_login` (`self.LoginUI`))) "Visible")
  (`Widget.SetVisibility` (`/Game/Maps/Login/BP_Login.UserList` (`/Game/Maps/Login/BP_UIManager.bp_login` (`self.LoginUI`))) "Visible")
  (`Widget.SetVisibility` (`/Game/Maps/Login/BP_Login.UserListBackGround` (`/Game/Maps/Login/BP_UIManager.bp_login` (`self.LoginUI`))) "Visible")
  (`Widget.SetVisibility` (`/Game/Maps/Login/BP_Login.UserListName` (`/Game/Maps/Login/BP_UIManager.bp_login` (`self.LoginUI`))) "Visible")
  (`Widget.SetVisibility` (`/Game/Maps/Login/BP_Login.UserListRoomButton` (`/Game/Maps/Login/BP_UIManager.bp_login` (`self.LoginUI`))) "Visible"))

(fn `UserConstructionScript`)